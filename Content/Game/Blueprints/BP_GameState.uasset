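; BP_GameState tracks level progression, collected bonuses and a per-level countdown for a multi-level game.
; A looping one-second timer calls LevelLost at zero, clearing that level's bonuses and restarting via BP_GameMode.
; LevelPassed banks bonuses and advances, or shows BP_HUD's game-over screen after the last level and resets to level one.
; Getters derive speed and start time from per-level maps, and trim the platform list by levels remaining.
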(event Custom|UpdateTimeLeft
  (bind _result (Math|Integer|DecrementInt (Variables|Default|GettimeLeft))
    (:%20%20
      (if (<= _result 0)
        (CallFunction|LevelLost)))))

(event EventBeginPlay
  (bind _starttime (CallFunction|GetCurrentLevelStartTime))
  (Variables|Default|SettimeLeft _starttime)
  (Utilities|Time|SetTimerbyEvent (delegate Custom|UpdateTimeLeft) 1.0 true)
  (bind _asbp_game_mode (Utilities|Casting|CastToBP_GameMode (Game|GetGameMode)))
  (Variables|Default|SetgameMode _asbp_game_mode))

(fn ConstructionScript)

(fn BonusCollected
  (Math|Integer|IncrementInt (Variables|Default|GetlevelCollectedBonusesCount)))

(fn LevelPassed
  (if (< (Variables|Default|Getlevel) (Variables|Default|GetmaxLevel))
    (Math|Integer|IncrementInt (Variables|Default|Getlevel)
      (:%20%20
        (Variables|Default|SettotalCollectedBonusesCount (+ (Variables|Default|GettotalCollectedBonusesCount) (Variables|Default|GetlevelCollectedBonusesCount)))
        (Variables|Default|SetlevelCollectedBonusesCount 0)))
    (else
      (bind _asbp_hud (Utilities|Casting|CastToBP_HUD (HUD|GetHUD (Game|GetPlayerController 0))))
      (Default|ShowGameOverScreen _asbp_hud (+ (Variables|Default|GettotalCollectedBonusesCount) (Variables|Default|GetlevelCollectedBonusesCount)))
      (Variables|Default|Setlevel 1)
      (Variables|Default|SettotalCollectedBonusesCount 0)
      (Variables|Default|SetlevelCollectedBonusesCount 0)))
  (CallFunction|ResetTimer)
  (Default|RestartLevel (Variables|Default|GetgameMode)))

(fn LevelLost
  (Variables|Default|SetlevelCollectedBonusesCount 0)
  (CallFunction|ResetTimer)
  (Default|RestartLevel (Variables|Default|GetgameMode)))

(fn ResetTimer
  (Utilities|Time|ClearTimerbyFunctionName 0 "UpdateTimeLeft")
  (bind _starttime (CallFunction|GetCurrentLevelStartTime))
  (Variables|Default|SettimeLeft _starttime)
  (Utilities|Time|SetTimerbyFunctionName 0 "UpdateTimeLeft" 1.0 true))

(fn GetCurrentLevelPlatforms
  (bind _platfroms (Variables|Default|Getplatfroms))
  (bind _res (LocalVariables|Getres))
  (for (_array_element _array_index) _platfroms
    (if (< _array_index (- (Utilities|Array|Length _platfroms) (- (Variables|Default|GetmaxLevel) (Variables|Default|Getlevel))))
      (Utilities|Array|Add _res _array_element)))
  (return _res))

(fn GetCurrentLevelSpeedCoef
  (return (.Value (Utilities|Map|Find (Variables|Default|GetspeedCoefByLevel) (Variables|Default|Getlevel)))))

(fn GetCurrentLevelStartTime
  (return (.Value (Utilities|Map|Find (Variables|Default|GetstartTimeByLevel) (Variables|Default|Getlevel)))))