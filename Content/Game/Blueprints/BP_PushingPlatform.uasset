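; BP_PushingPlatform is a platform with two walls that slide back and forth along relative Y in opposite directions.
; On BeginPlay it may spawn bonuses at four spawn points and divides the oscillation period by the GameState's level speed coefficient, so higher coefficients move faster.
; Tick accumulates time into a linear ping-pong between the Y bounds, applying it to one wall and its mirrored value to the other.
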(event EventBeginPlay
  (|CallParentFunction)
  (CallFunction|SpawnBonuses (Utilities|Array|MakeArray (Variables|Default|GetBonusSpawn1) (Variables|Default|GetBonusSpawn2) (Variables|Default|GetBonusSpawn3) (Variables|Default|GetBonusSpawn4)) 0.25)
  (bind _speedcoef (Default|GetCurrentLevelSpeedCoef (Variables|Default|GetgameState)))
  (Variables|Default|SetoscillationDuration (/ (Variables|Default|GetoscillationDuration) _speedcoef)))

(event EventTick
  (params (DeltaSeconds :type Float%20%28single-precision%29))
  (bind _oscillationduration (Variables|Default|GetoscillationDuration))
  (bind _movingwall2 (Variables|Default|GetMovingWall2))
  (bind _movingwall1 (Variables|Default|GetMovingWall1))
  (bind _returnvalue (/ _oscillationduration 2.0))
  (bind _relativelocation (Variables|/Script/Engine.SceneComponent|GetRelativeLocation _movingwall1))
  (bind _relativelocation_2 (Variables|/Script/Engine.SceneComponent|GetRelativeLocation _movingwall2))
  (Variables|Default|Settime (+ DeltaSeconds (Variables|Default|Gettime)))
  (if (>= (Math|Float|%(Float) (Variables|Default|Gettime) (Variables|Default|GetoscillationDuration)) _returnvalue)
    (Variables|Default|SettargetY (+ (Variables|Default|GetlowerBoundY) (* (- (Variables|Default|GetupperBoundY) (Variables|Default|GetlowerBoundY)) (/ (Math|Float|%(Float) (Variables|Default|Gettime) _returnvalue) _returnvalue))))
    (else
      (Variables|Default|SettargetY (- (Variables|Default|GetupperBoundY) (* (- (Variables|Default|GetupperBoundY) (Variables|Default|GetlowerBoundY)) (/ (Math|Float|%(Float) (Variables|Default|Gettime) _returnvalue) _returnvalue))))))
  (Utilities|FlowControl|Sequence
    (:then_0
      (Transformation|SetRelativeLocation _movingwall1 (Math|Vector|MakeVector (.x _relativelocation) (Variables|Default|GettargetY) (.z _relativelocation)) false false))
    (:then_1
      (Transformation|SetRelativeLocation _movingwall2 (Math|Vector|MakeVector (.x _relativelocation_2) (+ (- (Variables|Default|GetupperBoundY) (Variables|Default|GettargetY)) (Variables|Default|GetlowerBoundY)) (.z _relativelocation_2)) false false))))

(fn ConstructionScript
  (|CallParentFunction))