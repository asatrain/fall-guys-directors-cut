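; Level platform with four walls that move up and down in alternating pairs, plus bonus spawning at two spawn points.
; BeginPlay spawns the bonuses and divides the oscillation duration by the GameState's level speed coefficient, so walls move faster as that coefficient rises.
; Tick turns accumulated time into a linear triangle wave between the Z bounds, with Wall2 and Wall4 mirroring Wall1 and Wall3.
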(event EventBeginPlay
  (|CallParentFunction)
  (CallFunction|SpawnBonuses (Utilities|Array|MakeArray (Variables|Default|GetBonusSpawn1) (Variables|Default|GetBonusSpawn2)) 0.5)
  (bind _speedcoef (Default|GetCurrentLevelSpeedCoef (Variables|Default|GetgameState)))
  (Variables|Default|SetoscillationDuration (/ (Variables|Default|GetoscillationDuration) _speedcoef)))

(event EventTick
  (params (DeltaSeconds :type Float%20%28single-precision%29))
  (bind _oscillationduration (Variables|Default|GetoscillationDuration))
  (bind _wall1 (Variables|Default|GetWall1))
  (bind _wall2 (Variables|Default|GetWall2))
  (bind _wall4 (Variables|Default|GetWall4))
  (bind _wall3 (Variables|Default|GetWall3))
  (bind _returnvalue (/ _oscillationduration 2.0))
  (bind _relativelocation (Variables|/Script/Engine.SceneComponent|GetRelativeLocation _wall4))
  (bind _relativelocation_2 (Variables|/Script/Engine.SceneComponent|GetRelativeLocation _wall3))
  (bind _relativelocation_3 (Variables|/Script/Engine.SceneComponent|GetRelativeLocation _wall2))
  (bind _relativelocation_4 (Variables|/Script/Engine.SceneComponent|GetRelativeLocation _wall1))
  (Variables|Default|Settime (+ DeltaSeconds (Variables|Default|Gettime)))
  (if (>= (Math|Float|%(Float) (Variables|Default|Gettime) (Variables|Default|GetoscillationDuration)) _returnvalue)
    (Variables|Default|SettargetZ (+ (Variables|Default|GetlowerBoundZ) (* (- (Variables|Default|GetupperBoundZ) (Variables|Default|GetlowerBoundZ)) (/ (Math|Float|%(Float) (Variables|Default|Gettime) _returnvalue) _returnvalue))))
    (else
      (Variables|Default|SettargetZ (- (Variables|Default|GetupperBoundZ) (* (- (Variables|Default|GetupperBoundZ) (Variables|Default|GetlowerBoundZ)) (/ (Math|Float|%(Float) (Variables|Default|Gettime) _returnvalue) _returnvalue))))))
  (Utilities|FlowControl|Sequence
    (:then_0
      (Transformation|SetRelativeLocation _wall1 (Math|Vector|MakeVector (.x _relativelocation_4) (.y _relativelocation_4) (Variables|Default|GettargetZ)) false false))
    (:then_1
      (Transformation|SetRelativeLocation _wall3 (Math|Vector|MakeVector (.x _relativelocation_2) (.y _relativelocation_2) (Variables|Default|GettargetZ)) false false))
    (:then_2
      (Transformation|SetRelativeLocation _wall2 (Math|Vector|MakeVector (.x _relativelocation_3) (.y _relativelocation_3) (+ (- (Variables|Default|GetupperBoundZ) (Variables|Default|GettargetZ)) (Variables|Default|GetlowerBoundZ))) false false))
    (:then_3
      (Transformation|SetRelativeLocation _wall4 (Math|Vector|MakeVector (.x _relativelocation) (.y _relativelocation) (+ (- (Variables|Default|GetupperBoundZ) (Variables|Default|GettargetZ)) (Variables|Default|GetlowerBoundZ))) false false))))

(fn ConstructionScript
  (|CallParentFunction))