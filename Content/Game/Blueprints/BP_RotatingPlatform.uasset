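; BP_RotatingPlatform is a level obstacle or platform with three cylinders that spin continuously and can carry bonus pickups.
; On BeginPlay it spawns bonuses at three spawn points with a probability weight and scales its rotation speed by the GameState's current level speed coefficient.
; Tick applies a frame-rate-independent local yaw rotation to each cylinder using that speed.
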(event EventTick
  (params (DeltaSeconds :type Float%20%28single-precision%29))
  (for _array_element (Variables|Default|Getcylinders)
    (Transformation|AddLocalRotation _array_element (Math|Rotator|MakeRotator 0.0 0.0 (* (Variables|Default|GetrotateSpeed) (Utilities|Time|GetWorldDeltaSeconds))) false false)))

(event EventBeginPlay
  (|CallParentFunction)
  (Variables|Default|Setcylinders (Utilities|Array|MakeArray (Variables|Default|GetCylinder) (Variables|Default|GetCylinder1) (Variables|Default|GetCylinder2)))
  (CallFunction|SpawnBonuses (Utilities|Array|MakeArray (Variables|Default|GetBonusSpawn1) (Variables|Default|GetBonusSpawn2) (Variables|Default|GetBonusSpawn3)) 0.3)
  (bind _speedcoef (Default|GetCurrentLevelSpeedCoef (Variables|Default|GetgameState)))
  (Variables|Default|SetrotateSpeed (* _speedcoef (Variables|Default|GetrotateSpeed))))

(fn ConstructionScript
  (|CallParentFunction))