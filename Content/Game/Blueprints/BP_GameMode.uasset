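; Game mode that procedurally builds a level as a row of platforms at play start and on restart.
; Spawns a start platform, a series of random picks from the game state's current-level platform list with random yaw, then an end platform, spaced along X by platform widths.
; RestartLevel broadcasts LevelRestarting, moves the player character to the PlayerStart and generates a new layout.
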(event EventBeginPlay
  (bind _asbp_game_state (Utilities|Casting|CastToBP_GameState (Game|GetGameState)))
  (Variables|Default|SetbpGameState _asbp_game_state)
  (CallFunction|GeneratePlatforms))

(fn ConstructionScript)

(fn RestartLevel
  (Default|CallLevelRestarting)
  (bind _returnvalue (Actor|GetActorOfClass "/Script/Engine.PlayerStart"))
  (Transformation|SetActorTransform (Game|GetPlayerCharacter 0) (Transformation|GetActorTransform _returnvalue))
  (CallFunction|GeneratePlatforms))

(fn GeneratePlatforms
  (bind _returnvalue (Game|SpawnActorfromClass "/Game/Game/Blueprints/BP_StartPlatform.BP_StartPlatform_C" (Math|Transform|MakeTransform "0, 0, 0" "0, 0, 0" "1,1,1") "Undefined" 0 0))
  (Utilities|Array|Add (Variables|Default|GetgeneratedPlatforms) _returnvalue)
  (bind _platfroms (Default|GetCurrentLevelPlatforms (Variables|Default|GetbpGameState)))
  (for _index (range 0 (- (Variables|Default|GetplatfromsCount) 1))
    (bind _returnvalue_2 (Game|SpawnActorfromClass (.OutItem (Utilities|Array|Random _platfroms)) (Math|Transform|MakeTransform (Math|Vector|MakeVector (+ (+ (* _index (Variables|Default|GetplatfromWidth)) (/ (Variables|Default|GetstartEndPlatformWidth) 2.0)) (/ (Variables|Default|GetplatfromWidth) 2.0)) 0.0 0.0) (Math|Rotator|MakeRotator 0.0 0.0 (.OutItem (Utilities|Array|Random (LocalVariables|GetspawnRotationsZ)))) "1,1,1") "Undefined" 0 0))
    (Utilities|Array|Add (Variables|Default|GetgeneratedPlatforms) _returnvalue_2))
  (bind _returnvalue_3 (Game|SpawnActorfromClass "/Game/Game/Blueprints/BP_EndPlatform.BP_EndPlatform_C" (Math|Transform|MakeTransform (Math|Vector|MakeVector (+ (Variables|Default|GetstartEndPlatformWidth) (* (Variables|Default|GetplatfromsCount) (Variables|Default|GetplatfromWidth))) 0.0 0.0) "0, 0, 0" "1,1,1") "Undefined" 0 0))
  (Utilities|Array|Add (Variables|Default|GetgeneratedPlatforms) _returnvalue_3))